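; Tile map actor that serves as the game's grid, tracking walls and creatures for movement checks and spawning.
; On BeginPlay it flags layer-1 tiles as blocked in a flat boolean array, sends the knight to a random cell and shows the kill-count UI.
; CanGo rejects out-of-bounds, wall and creature-occupied cells, backing a random-retry spawn picker.
; SpawnMob and Despawn maintain the creature list, with despawns notifying the spawner.
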(event `self.ReceiveBeginPlay`
  (bind (`_좌표_x` `_좌표_y`) (break `/Game/Blueprints/Struct/E_Grid_Position` (`self.Random Spawn`)))
  (bind _tilemap (`PaperTileMapComponent.TileMap` (`self.RenderComponent`)))
  (bind _mapheight (`PaperTileMap.MapHeight` _tilemap))
  (bind _mapwidth (`PaperTileMap.MapWidth` _tilemap))
  (`|ExecutionSequence`
    (:`then_0`
      (set `self.MapWidth` _mapwidth)
      (set `self.MapHeight` _mapheight)
      (`KismetArrayLibrary.Array_Resize` (`self.Map Grid`) (* _mapwidth _mapheight)))
    (:`then_1`
      (for (_ _array_index) (`self.Map Grid`)
        (bind (_returnvalue_tileindex _returnvalue_tileset) (break `PaperTileInfo` (`PaperTileMapComponent.GetTile` (`self.RenderComponent`) (mod _array_index (`self.MapWidth`)) (/ _array_index (`self.MapHeight`)) 1)))
        (`/Engine/EditorBlueprintResources/StandardMacros.IsValid` _returnvalue_tileset ; 앞선 조건과 같은 것들 모두
          (:`Is Valid`
            (`KismetArrayLibrary.Array_Set` (`self.Map Grid`) _array_index true) ; 트루 값으로 반환
          ))))
    (:`then_2`
      (bind _returnvalue (`GameplayStatics.GetActorOfClass` "/Game/Blueprints/Creatures/BP_Knight.BP_Knight_C"))
      (`/Game/Blueprints/Creatures/BP_Creature.Set_Destination` _returnvalue `_좌표_x` `_좌표_y` false)
      (`KismetArrayLibrary.Array_Add` (`self.Creature`) _returnvalue))
    (:`then_3`
      (bind _returnvalue_2 (`|CreateWidget` "/Game/Blueprints/UI/WBP_Kills_UI.WBP_Kills_UI_C"))
      (bind _output_get (set `self.Kill Count UI` _returnvalue_2))
      (`UserWidget.AddToViewport` _output_get 0))))

(fn `Can Go`
  (params (`Grid X` :type Integer) (`Grid Y` :type Integer))
  (returns (Can :type Boolean))
  (bind (_vaild _index) (`self.Grid Position To Index` `Grid X` `Grid Y`))
  (if _vaild
    (if (not (`|GetArrayItem` (`self.Map Grid`) _index))
      (bind _found (`self.크리처 존재 여부` `Grid X` `Grid Y`))
      (return (not _found))
      (else
        _)))
  (return false))

(fn `Despawn`
  (params (`Despawn Creature` :type "/Game/Blueprints/Creatures/BP_Creature Object Reference"))
  (`/Engine/EditorBlueprintResources/StandardMacros.IsValid` `Despawn Creature`
    (:`Is Valid`
      (`KismetArrayLibrary.Array_RemoveItem` (`self.Creature`) `Despawn Creature`)
      (`self.K2_DestroyActor` `Despawn Creature`)
      (`/Game/Blueprints/BP_Spawning.OnDespawnMob` (`self.BP_Spawning`)))))

(fn `Get Tile Position`
  (params (`Grid X` :type Integer) (`Grid Y` :type Integer))
  (returns (Valid :type Boolean) (Location :type "Vector Structure"))
  (bind _vaild (`self.Grid Position To Index` `Grid X` `Grid Y`))
  (return _vaild (+ (`self.K2_GetActorLocation`) (`KismetMathLibrary.MakeVector` (* `Grid X` (`self.Tile X`) 5.0) 0.0 (* `Grid Y` (`self.Tile Y`) -5.0)))))

(fn `Grid Position To Index`
  (params (`Grid X` :type Integer) (`Grid Y` :type Integer))
  (returns (Vaild :type Boolean) (Index :type Integer))
  (return (and (`KismetMathLibrary.InRange_IntInt` `Grid X` 0 (`self.MapWidth`) true false) (`KismetMathLibrary.InRange_IntInt` `Grid Y` 0 (`self.MapHeight`) true false)) (+ `Grid X` (* `Grid Y` (`self.MapWidth`)))))

(fn `Random Spawn`
  (returns (`좌표` :type "/Game/Blueprints/Struct/E_Grid_Position Structure"))
  (locals (`랜덤 위치` :type "/Game/Blueprints/Struct/E_Grid_Position Structure"))
  (for _ (range 1001)
    (bind _output_get (set `local.랜덤 위치` (make `/Game/Blueprints/Struct/E_Grid_Position` (`KismetMathLibrary.RandomIntegerInRange` 0 (- (`self.MapWidth`) 1)) (`KismetMathLibrary.RandomIntegerInRange` 0 (- (`self.MapHeight`) 1)))))
    (bind _can (`self.Can Go` (break `/Game/Blueprints/Struct/E_Grid_Position` _output_get) (`.Y_4_2659769B4A6BDAD04D86A9BD02D0E451` (break `/Game/Blueprints/Struct/E_Grid_Position` _output_get))))
    (if _can
      (break)))
  (return (`local.랜덤 위치`)))

(fn `Spawn mob`
  (params (`스폰 몬스터` :type "/Game/Blueprints/Creatures/BP_Creature Class Reference"))
  (bind (`_좌표_x` `_좌표_y`) (break `/Game/Blueprints/Struct/E_Grid_Position` (`self.Random Spawn`)))
  (bind (_valid _location) (`self.Get Tile Position` `_좌표_x` `_좌표_y`))
  (if _valid
    (bind _returnvalue (`|SpawnActorFromClass` `스폰 몬스터` (`KismetMathLibrary.MakeTransform` (`KismetMathLibrary.MakeVector` (.x _location) 5.0 (.z _location))) "Undefined" "MultiplyWithRoot" null null))
    (`/Game/Blueprints/Creatures/BP_Creature.Set_Destination` _returnvalue `_좌표_x` `_좌표_y` false)
    (`KismetArrayLibrary.Array_Add` (`self.Creature`) _returnvalue)))

(fn `UserConstructionScript`)

(fn `크리처 존재 여부`
  (params (`Grid X` :type Integer) (`Grid Y` :type Integer))
  (returns (Found :type Boolean) (Creature :type "/Game/Blueprints/Creatures/BP_Creature Object Reference"))
  (for _array_element (`self.Creature`)
    (bind (_gridposition_x _gridposition_y) (break `/Game/Blueprints/Struct/E_Grid_Position` (`/Game/Blueprints/Creatures/BP_Creature.GridPosition` _array_element)))
    (if (and (== _gridposition_x `Grid X`) (== _gridposition_y `Grid Y`))
      (return true _array_element)))
  (return false null) ; 찾아내지 못한 경우
)