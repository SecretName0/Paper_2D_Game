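; BP_Spawning keeps the BP_TileMap that owns it populated with BP_Skeleton mobs, up to a maximum count.
; On BeginPlay it caches the owning tile map and starts a self-recalling spawn loop.
; The loop reserves a slot, waits a random delay and calls the map's SpawnMob, or rechecks each tick while at the cap.
; OnDespawnMob decrements the count, freeing a slot for another spawn.
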(event `self.ReceiveBeginPlay`
  (bind _asbp_tile_map (cast `/Game/Blueprints/BP_TileMap` (`self.GetOwner`)))
  (set `self.Tile Map` _asbp_tile_map)
  (`self.Tick Random Spawn`))

(event `Tick Random Spawn`
  (if (< (`self.몹의 수`) (`self.몹 최대치`))
    (`/Engine/EditorBlueprintResources/StandardMacros.IncrementInt` (`self.몹의 수`)
      (:`  `
        (`KismetSystemLibrary.Delay` (`KismetMathLibrary.RandomFloatInRange` 0.0 10.0))
        (`/Game/Blueprints/BP_TileMap.Spawn mob` (`self.Tile Map`) "/Game/Blueprints/Creatures/BP_Skeleton.BP_Skeleton_C")
        (`self.Tick Random Spawn`)))
    (else
      (`KismetSystemLibrary.DelayUntilNextTick`)
      (`self.Tick Random Spawn`))))

(fn `OnDespawnMob`
  (`/Engine/EditorBlueprintResources/StandardMacros.DecrementInt` (`self.몹의 수`)))