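; AI controller for BP_Monsters creatures that finds the BP_Knight player and triggers melee-range attacks.
; It caches the possessed monster and runs a simple state switch on the monster's State every Tick.
; Idle looks up the knight by class, sets it as target and switches to Move.
; Move waits until the monster reaches its destination, faces the target and fires AttackEvent when within one tile.
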(event `self.ReceivePossess`
  (params (PossessedPawn :type "Pawn Object Reference"))
  (bind _asbp_monsters (cast `/Game/Blueprints/Creatures/BP_Monsters` PossessedPawn))
  (set `self.몬스터` _asbp_monsters))

(event `self.ReceiveTick`
  (params (DeltaSeconds :type "Float (single-precision)"))
  (`self.AI_Input`))

(fn `AI_Input`
  (bind `_몬스터` (`self.몬스터`))
  (bind `_몬스터_2` (`self.몬스터`))
  (bind `_타겟` (`/Game/Blueprints/Creatures/BP_Monsters.타겟` `_몬스터_2`))
  (switch `/Game/Blueprints/Struct/E_State` (`/Game/Blueprints/Creatures/BP_Creature.State` (`self.몬스터`))
    (:`NewEnumerator0`
      ;[1 1 1] 대기할 때
      (bind _returnvalue (`GameplayStatics.GetActorOfClass` "/Game/Blueprints/Creatures/BP_Knight.BP_Knight_C")) ; 플레이어를 발견
      (bind _output_get (set `/Game/Blueprints/Creatures/BP_Monsters.타겟` _returnvalue `_몬스터_2`))
      (`/Engine/EditorBlueprintResources/StandardMacros.IsValid` _output_get ; 발견하였을 때
        (:`Is Valid`
          (set `/Game/Blueprints/Creatures/BP_Creature.State` "NewEnumerator1" (`self.몬스터`)))))
    (:`NewEnumerator1`
      ;[1 1 1] move상태
      (`/Engine/EditorBlueprintResources/StandardMacros.IsValid` `_타겟`
        (:`Is Valid`
          (if (`/Game/Blueprints/Creatures/BP_Creature.목적지 도달 여부` `_몬스터_2`)
            (`/Game/Blueprints/Creatures/BP_Creature.Look At Target` `_몬스터` `_타겟`)
            (bind _count (`/Game/Blueprints/Creatures/BP_Creature.Get Tile Count to Target` `_몬스터` `_타겟`))
            (if (<= _count 1)
              (`/Game/Blueprints/Creatures/BP_Creature.Attack Event` (`self.몬스터`)))))))))

(fn `UserConstructionScript`)