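; Paper2D creature with four-direction movement, melee attack and health, with stats and flipbooks read from Data.
; Tick applies movement input on the XZ plane and picks a flipbook from State and Direction, rotating the side sprite to face left.
; AttackEvent damages other creatures overlapping the directional hit area, then returns to Idle after the animation's length.
; OnDamaged clamps HP and updates the health bar widget.
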(event `self.ReceiveTick`
  (params (DeltaSeconds :type "Float (single-precision)"))
  (`self.Moving Logic`)
  (`self.Update Animation`))

(event `self.ReceiveBeginPlay`
  (bind _data_hp (break `/Game/Blueprints/Data/Creature_Data` (`self.Data`)))
  (bind _output_get (set `self.HP` _data_hp))
  (set `self.Max_HP` _output_get))

(event `Attack Event`
  (switch `/Game/Blueprints/Struct/E_State` (`self.State`)
    (:`NewEnumerator0`
      _)
    (:`NewEnumerator1`
      _))
  (set `self.State` "NewEnumerator2")
  (`self.Update Animation`)
  (`self.Process Attack`)
  (`KismetSystemLibrary.Delay` (`PaperFlipbookComponent.GetFlipbookLength` (`self.Sprite`)))
  (set `self.State` "NewEnumerator0"))

(fn `Moving Logic`
  (switch `/Game/Blueprints/Struct/E_State` (`self.State`)
    (:`NewEnumerator1`
      (`self.AddMovementInput` (select `/Game/Blueprints/Struct/E_Direction` (`self.Direction`) :`NewEnumerator0` (0.0 0.0 1.0) :`NewEnumerator1` (0.0 0.0 -1.0) :`NewEnumerator2` (1.0 0.0 0.0) :`NewEnumerator3` (-1.0 0.0 0.0) :!type "Vector Structure")))))

(fn `On Damaged`
  (params (Damaged :type Integer) (Attacker :type "/Game/Blueprints/Creatures/BP_Creature Object Reference"))
  (locals (NewLocalVar :type "ProgressBar Object Reference"))
  (bind _max_hp (`self.Max_HP`))
  (if (not (== Attacker self))
    (bind _output_get (set `self.HP` (`KismetMathLibrary.Clamp` (- (`self.HP`) Damaged) 0 _max_hp)))
    (bind _aswbp_hp_bar (cast `/Game/Blueprints/UI/WBP_HpBar` (`WidgetComponent.GetUserWidgetObject` (`self.HP_Widget`))))
    (set `/Game/Blueprints/UI/WBP_HpBar.HpRatio` (/ _output_get (`KismetMathLibrary.Conv_IntToDouble` _max_hp)) _aswbp_hp_bar)))

(fn `Process Attack`
  (bind (_data_hp _data_damage) (break `/Game/Blueprints/Data/Creature_Data` (`self.Data`)))
  (bind `_공격_범위_좌우_` (`self.공격 범위[좌우]`))
  (for _array_element (`PrimitiveComponent.GetOverlappingActors` (select `/Game/Blueprints/Struct/E_Direction` (`self.Direction`) :`NewEnumerator0` (`self.공격 범위[상단]`) :`NewEnumerator1` (`self.공격 범위[하단]`) :`NewEnumerator2` `_공격_범위_좌우_` :`NewEnumerator3` `_공격_범위_좌우_`) "BP_Creature_C")
    (bind _asbp_creature (cast `/Game/Blueprints/Creatures/BP_Creature` _array_element))
    (if (not (== _asbp_creature self))
      (`self.On Damaged` _asbp_creature _data_damage self))))

(fn `Update Animation`
  (bind (_data_hp _data_damage _data_up_idle _data_down_idle _data_side_idle _data_up_move _data_down_move _data_side_move _data_up_attack _data_down_attack _data_side_attack) (break `/Game/Blueprints/Data/Creature_Data` (`self.Data`)))
  (`SceneComponent.K2_SetRelativeRotation` (`self.Sprite`) (select `bool` (`|EnumEquality` (`self.Direction`) "NewEnumerator3") :`true` (struct :`Yaw` 180.0) :!type "Rotator Structure") false false)
  (switch `/Game/Blueprints/Struct/E_State` (`self.State`)
    (:`NewEnumerator0`
      (`PaperFlipbookComponent.SetFlipbook` (`self.Sprite`) (select `/Game/Blueprints/Struct/E_Direction` (`self.Direction`) :`NewEnumerator0` _data_up_idle :`NewEnumerator1` _data_down_idle :`NewEnumerator2` _data_side_idle :`NewEnumerator3` _data_side_idle)))
    (:`NewEnumerator1`
      (`PaperFlipbookComponent.SetFlipbook` (`self.Sprite`) (select `/Game/Blueprints/Struct/E_Direction` (`self.Direction`) :`NewEnumerator0` _data_up_move :`NewEnumerator1` _data_down_move :`NewEnumerator2` _data_side_move :`NewEnumerator3` _data_side_move)))
    (:`NewEnumerator2`
      (`PaperFlipbookComponent.SetFlipbook` (`self.Sprite`) (select `/Game/Blueprints/Struct/E_Direction` (`self.Direction`) :`NewEnumerator0` _data_up_attack :`NewEnumerator1` _data_down_attack :`NewEnumerator2` _data_side_attack :`NewEnumerator3` _data_side_attack)))))

(fn `UserConstructionScript`)