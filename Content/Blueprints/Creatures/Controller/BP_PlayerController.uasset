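; Player controller that turns movement input into state and facing direction for the BP_Knight pawn it controls.
; BeginPlay caches the possessed knight, and Tick runs InputData every frame.
; While the knight is Idle or Move, InputData sets Move or Idle from the forward/back and left/right axes, then sets Direction from each axis sign.
; The left/right check runs last, so it wins on diagonal input.
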(event `self.ReceiveBeginPlay`
  ;[1 1 1] 컨트롤 대상 확인
  (bind _asbp_knight (cast `/Game/Blueprints/Creatures/BP_Knight` (`self.K2_GetPawn`)))
  (set `self.플레이어` _asbp_knight))

(event `self.ReceiveTick`
  (params (DeltaSeconds :type "Float (single-precision)"))
  (`self.Input_Data`))

(fn `Input_Data`
  (bind `_플레이어` (`self.플레이어`))
  (switch `/Game/Blueprints/Struct/E_State` (`/Game/Blueprints/Creatures/BP_Creature.State` (`self.플레이어`))
    (:`NewEnumerator0`
      _)
    (:`NewEnumerator1`
      _))
  (`|ExecutionSequence`
    (:`then_0`
      (if (or (!= (`self.GetInputAxisValue`) 0.0) (!= (`self.GetInputAxisValue`) 0.0))
        (set `/Game/Blueprints/Creatures/BP_Creature.State` "NewEnumerator1" `_플레이어`)
        (else
          (set `/Game/Blueprints/Creatures/BP_Creature.State` "NewEnumerator0" `_플레이어`))))
    (:`then_1`
      (`/Engine/EditorBlueprintResources/StandardMacros.CompareFloat` (`self.GetInputAxisValue`) ; 값 비교
        (:`>`
          (set `/Game/Blueprints/Creatures/BP_Creature.Direction` "NewEnumerator0" `_플레이어`))
        (:`<`
          (set `/Game/Blueprints/Creatures/BP_Creature.Direction` "NewEnumerator1" `_플레이어`))))
    (:`then_2`
      (`/Engine/EditorBlueprintResources/StandardMacros.CompareFloat` (`self.GetInputAxisValue`) ; 값 비교
        (:`>`
          (set `/Game/Blueprints/Creatures/BP_Creature.Direction` "NewEnumerator2" `_플레이어`))
        (:`<`
          (set `/Game/Blueprints/Creatures/BP_Creature.Direction` "NewEnumerator3" `_플레이어`))))))

(fn `UserConstructionScript`)