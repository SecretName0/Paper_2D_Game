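; BP_Creature is a Paper2D creature with HP, a four-direction facing and Idle, Move and Attack states.
; UpdateAnimation picks flipbooks from Data by state and direction, mirroring side sprites for Left via rotation, while MovingLogic applies directional movement input during Move.
; AttackEvent damages other creatures overlapping the attack range through OnDamaged, which clamps HP, then returns to Idle after the flipbook's length.
; Direction-from-input comparisons sit unconnected in the EventGraph.
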(event `Attack Event`
  (switch `/Game/Blueprints/E_State` (`self.State`)
    (:`NewEnumerator0`
      _)
    (:`NewEnumerator1`
      _))
  (set `self.State` "NewEnumerator2")
  (`self.Update Animation`)
  (`self.Process Attack`)
  (`KismetSystemLibrary.Delay` (`PaperFlipbookComponent.GetFlipbookLength` (`self.Sprite`)))
  (set `self.State` "NewEnumerator0"))

(fn `Moving Logic`
  (switch `/Game/Blueprints/E_State` (`self.State`)
    (:`NewEnumerator1`
      (`self.AddMovementInput` (select `/Game/Blueprints/E_Direction` (`self.Direction`) :`NewEnumerator0` (0.0 0.0 1.0) :`NewEnumerator1` (0.0 0.0 -1.0) :`NewEnumerator2` (1.0 0.0 0.0) :`NewEnumerator3` (-1.0 0.0 0.0) :!type "Vector Structure")))))

(fn `On Damaged`
  (params (Damaged :type Integer) (Attacker :type "/Game/Blueprints/BP_Creature Object Reference"))
  (if (not (== Attacker self))
    (set `self.HP` (`KismetMathLibrary.Clamp` (- (`self.HP`) Damaged) 0 (`self.Max_HP`)))))

(fn `Process Attack`
  (for _array_element (`PrimitiveComponent.GetOverlappingActors` (`self.공격 범위`) "BP_Creature_C")
    (bind _asbp_creature (cast `/Game/Blueprints/BP_Creature` _array_element))
    (if (not (== _asbp_creature self))
      (`self.On Damaged` _asbp_creature 25 self)
      (`KismetSystemLibrary.PrintText` (`KismetTextLibrary.Conv_IntToText` (`/Game/Blueprints/BP_Creature.HP` _asbp_creature))))))

(fn `Update Animation`
  (bind (_data_up_idle _data_down_idle _data_side_idle _data_up_move _data_down_move _data_side_move _data_up_attack _data_down_attack _data_side_attack) (break `/Game/Blueprints/Data/Creature_Data` (`self.Data`)))
  (`SceneComponent.K2_SetRelativeRotation` (`self.Sprite`) (select `bool` (`|EnumEquality` (`self.Direction`) "NewEnumerator3") :`true` (struct :`Yaw` 180.0) :!type "Rotator Structure") false false)
  (switch `/Game/Blueprints/E_State` (`self.State`)
    (:`NewEnumerator0`
      (`PaperFlipbookComponent.SetFlipbook` (`self.Sprite`) (select `/Game/Blueprints/E_Direction` (`self.Direction`) :`NewEnumerator0` _data_up_idle :`NewEnumerator1` _data_down_idle :`NewEnumerator2` _data_side_idle :`NewEnumerator3` _data_side_idle)))
    (:`NewEnumerator1`
      (`PaperFlipbookComponent.SetFlipbook` (`self.Sprite`) (select `/Game/Blueprints/E_Direction` (`self.Direction`) :`NewEnumerator0` _data_up_move :`NewEnumerator1` _data_down_move :`NewEnumerator2` _data_side_move :`NewEnumerator3` _data_side_move)))
    (:`NewEnumerator2`
      (`PaperFlipbookComponent.SetFlipbook` (`self.Sprite`) (select `/Game/Blueprints/E_Direction` (`self.Direction`) :`NewEnumerator0` _data_up_attack :`NewEnumerator1` _data_down_attack :`NewEnumerator2` _data_side_attack :`NewEnumerator3` _data_side_attack)))))

(fn `UserConstructionScript`)