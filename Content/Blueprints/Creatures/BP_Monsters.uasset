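; Monster creature Blueprint that hunts the BP_Knight player, running a small state-machine AI every Tick after the parent's logic.
; Idle grabs the knight as target and switches to Move once it is valid.
; Move fires AttackEvent within the recognition range; otherwise it sets one of four Direction values from the dominant X or Z axis toward the target, chasing on the XZ plane.
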(event `self.ReceiveBeginPlay`
  (`parent.ReceiveBeginPlay`))

(event `self.ReceiveTick`
  (params (DeltaSeconds :type "Float (single-precision)"))
  (`parent.ReceiveTick` DeltaSeconds)
  (`self.AI`))

(fn `AI`
  (bind `_타겟` (`self.타겟`))
  (bind (`_추격_x` `_추격_y` `_추격_z`) (`KismetMathLibrary.BreakVector` (`self.추격`)))
  (switch `/Game/Blueprints/Struct/E_State` (`self.State`)
    (:`NewEnumerator0`
      ;[1 1 1] 대기할 때
      (bind _returnvalue (`GameplayStatics.GetActorOfClass` "/Game/Blueprints/Creatures/BP_Knight.BP_Knight_C")) ; 플레이어를 발견
      (bind _output_get (set `self.타겟` _returnvalue)) ; 타겟으로 설정
      (`/Engine/EditorBlueprintResources/StandardMacros.IsValid` _output_get ; 발견하였을 때
        (:`Is Valid`
          (set `self.State` "NewEnumerator1") ; move상태로 전환
        )))
    (:`NewEnumerator1`
      ;[1 1 1] move상태
      (`/Engine/EditorBlueprintResources/StandardMacros.IsValid` `_타겟`
        (:`Is Valid`
          (bind _output_get_2 (set `self.추격` (- (`self.K2_GetActorLocation` `_타겟`) (`self.K2_GetActorLocation`))))
          (if (< (`KismetMathLibrary.VSize` _output_get_2) (`self.몬스터 인식 유효 거리`))
            (`self.Attack Event`) ; 플레이어가 지정한 거리 300 이내에 있을 경우\n공격 애니메이션을 실행
            (elif (> (`KismetMathLibrary.Abs` `_추격_x`) (`KismetMathLibrary.Abs` `_추격_z`))
              (`/Engine/EditorBlueprintResources/StandardMacros.CompareFloat` `_추격_x`
                (:`>`
                  (set `self.Direction` "NewEnumerator2"))
                (:`<`
                  (set `self.Direction` "NewEnumerator3")))
              (else
                (`/Engine/EditorBlueprintResources/StandardMacros.CompareFloat` `_추격_z`
                  (:`>`
                    (set `self.Direction` "NewEnumerator0"))
                  (:`<`
                    (set `self.Direction` "NewEnumerator1")))))))))))

(fn `UserConstructionScript`
  (`parent.UserConstructionScript`))