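; BP_Knight is a player-controlled knight with movement and a basic attack, driven by a simple state and a four-way facing direction.
; Each tick it runs UpdateInput, MovingLogic and UpdateAnimation in order, while the basic attack input calls AttackEvent.
; UpdateInput switches between Idle and Move from the two movement axes only while in those states.
; It also sets Direction from the axis signs, with left/right overriding forward/back on diagonals.
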(event `self.ReceiveTick`
  (params (DeltaSeconds :type "Float (single-precision)"))
  (`self.Update_Input`)
  (`self.Moving_Logic`)
  (`self.Update Animation`))

(event `InputAction|기본 공격`
  (params (Key :type "Key Structure"))
  (:`Pressed`
    (`self.Attack Event`)))

(fn `Update_Input`
  (switch `/Game/Blueprints/E_State` (`self.State`)
    (:`NewEnumerator0`
      _)
    (:`NewEnumerator1`
      _))
  (`|ExecutionSequence`
    (:`then_0`
      (if (or (!= (`self.GetInputAxisValue`) 0.0) (!= (`self.GetInputAxisValue`) 0.0))
        (set `self.State` "NewEnumerator1")
        (else
          (set `self.State` "NewEnumerator0"))))
    (:`then_1`
      (`/Engine/EditorBlueprintResources/StandardMacros.CompareFloat` (`self.GetInputAxisValue`) ; 값 비교
        (:`>`
          (set `self.Direction` "NewEnumerator0"))
        (:`<`
          (set `self.Direction` "NewEnumerator1"))))
    (:`then_2`
      (`/Engine/EditorBlueprintResources/StandardMacros.CompareFloat` (`self.GetInputAxisValue`) ; 값 비교
        (:`>`
          (set `self.Direction` "NewEnumerator2"))
        (:`<`
          (set `self.Direction` "NewEnumerator3"))))))

(fn `UserConstructionScript`)